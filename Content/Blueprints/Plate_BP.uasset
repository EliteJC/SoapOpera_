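; Plate actor that prepares its static mesh materials and an unwrap render target at BeginPlay.
; It creates a dynamic instance of Plate_Inst for every material slot and stores them in MaterialInstances.
; It then creates a square render target as RTUnwrap and sets the SceneCaptureComponent2D texture target to None.
; Nothing here binds RTUnwrap to the capture or materials, and the construction script is empty.
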(event `self.ReceiveBeginPlay`
  (for _index (range (`PrimitiveComponent.GetNumMaterials` (`self.StaticMesh`)))
    (bind _returnvalue (`PrimitiveComponent.CreateDynamicMaterialInstance` (`self.StaticMesh`) _index "/Game/Art/Materials/Instances/Plate_Inst.Plate_Inst" "None"))
    (`KismetArrayLibrary.Array_Add` (`self.Material Instances`) _returnvalue))
  (`|ExecutionSequence`
    (:`then_0`
      (bind _returnvalue_2 (`KismetRenderingLibrary.CreateRenderTarget2D` 1024 1024))
      (set `self.RT Unwrap` _returnvalue_2)
      (set `SceneCaptureComponent2D.TextureTarget` null (`self.SceneCaptureComponent2D`)))))

(fn `UserConstructionScript`)