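; FPS_Cleaner is a first-person power-washing Blueprint that adds the Powerwash input mapping on BeginPlay and traces whenever Wash_IA triggers.
; CreateLineTraces lays out a row of parallel traces mirrored about the camera center, spaced by BrushRadius.
; MakeLineVector rotates the camera's right vector around its forward axis to angle the row.
; Each multi line trace uses the Visibility channel with debug drawing, and its hits are not yet processed.
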(event `self.ReceiveBeginPlay`
  (`EnhancedInputSubsystemInterface.AddMappingContext` (pcsubsystem `EnhancedInputLocalPlayerSubsystem` (`GameplayStatics.GetPlayerController` 0)) "/Game/Blueprints/Washing/Input/Powerwash_IMC.Powerwash_IMC" 0 (struct)))

(event `EnhancedInput|/Game/Blueprints/Washing/Input/Wash_IA`
  (params (ActionValue :type Boolean) (ElapsedSeconds :type "Float (double-precision)") (TriggeredSeconds :type "Float (double-precision)") (InputAction :type "InputAction Object Reference" :default "/Game/Blueprints/Washing/Input/Wash_IA.Wash_IA"))
  (:`Triggered`
    (`self.CreateLineTraces`)))

(fn `CreateLineTraces`
  (locals (`L-Index` :type Integer))
  (bind (_start _end) (`self.LineTraceForward` (* (`self.MakeLineVector`) (* (`local.L-Index`) (* (`self.BrushRadius`) -2.2))) 1500.0))
  (bind (_start_2 _end_2) (`self.LineTraceForward` (* (`self.MakeLineVector`) (* (`local.L-Index`) (* (`self.BrushRadius`) 2.2))) 1500.0))
  (for _index (range (+ (`self.Length`) 1))
    (set `local.L-Index` _index)
    (`|ExecutionSequence`
      (:`then_0`
        (`self.LineTraceForTargets` _start_2 _end_2))
      (:`then_1`
        (if (!= (`local.L-Index`) 0)
          (`self.LineTraceForTargets` _start _end))))))

(fn `LineTraceForTargets`
  (params (Start :type "Vector Structure") (End :type "Vector Structure"))
  (`KismetSystemLibrary.LineTraceMulti` :`Start` Start :`End` End :`TraceChannel` "TraceTypeQuery1" :`DrawDebugType` "ForDuration"))

(fn `UserConstructionScript`
  (`parent.UserConstructionScript`))